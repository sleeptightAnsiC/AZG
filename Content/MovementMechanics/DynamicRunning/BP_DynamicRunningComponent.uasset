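; Character component for dynamic running that ramps MaxWalkSpeed up or down toward a target speed for the current running state.
; Each tick it adjusts speed, then derives the state from ground contact, capsule height change, forward movement and sprint input.
; Per-state maps, key-checked on BeginPlay, supply speeds and ramp rates.
; A Niagara emitter, attached to the aiming component in its OnRep, toggles visibility by state.
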(event `self.ReceiveBeginPlay`
  (`self.CheckIfEveryMapContainAllParameters`)
  (`self.Set_OwningCharacter` (`self.GetOwner`)))

(event `self.ReceiveTick`
  (params (DeltaSeconds :type "Float (single-precision)"))
  (bind _new_walk_speed (`self.Tick_FindNewWalkSpeed` DeltaSeconds))
  (set `CharacterMovementComponent.MaxWalkSpeed` _new_walk_speed (`self.CharacterMovementRef`))
  (bind _newrunningstate (`self.FindNewRunningState`))
  (set `self.RunningState` _newrunningstate)
  (`self.ResolveEmiterVisibility`)
  (`self.DebugVariables` false))

(event `InputAxis|MoveForward` :consume false :overrideparent false
  (params (AxisValue :type "Float (single-precision)"))
  ;[1 1 1] Input logic
  (bind _ismoving_ (`self.IsOwnerMoving` AxisValue))
  (set `self.bMoving` _ismoving_))

(event `InputAction|Sprint`
  (params (Key :type "Key Structure"))
  ;[1 1 1] Input logic
  (:`Pressed`
    (set `self.bSprintKeyDown` true))
  (:`Released`
    (set `self.bSprintKeyDown` false)))

(fn `CheckIfContainsEveryKey`
  (params (TargetMap :type "Map of /Game/MovementMechanics/DynamicRunning/ERunningState Enum to Float (double-precision) (by ref)") (MapName :type String))
  (returns (`Valid?` :type Boolean))
  (locals (`(Local) Valid?` :type Boolean :default true))
  (bind _enumvalue (foreach `/Game/MovementMechanics/DynamicRunning/ERunningState` false)
    (:`LoopBody`
      (if (not (`BlueprintMapLibrary.Map_Contains` TargetMap _enumvalue))
        (set `local.(Local) Valid?` false)
        (bind _returnvalue (`KismetStringLibrary.Concat_StrStr` "ERROR!   " (`KismetSystemLibrary.GetDisplayName` self) ": " MapName " map (E_RunningState) does not contain key: " (`|GetEnumeratorNameAsString` _enumvalue)))
        (`KismetSystemLibrary.PrintString` _returnvalue true true (struct :`R` 0.779167 :`B` 0.048325 :`A` 1.0) 10.0 (`KismetStringLibrary.Conv_StringToName` _returnvalue))))
    (:`then`
      (return (`local.(Local) Valid?`)))))

(fn `CheckIfEveryMapContainAllParameters`
  (returns (`Success?` :type Boolean))
  (locals (`(Local) Success?` :type Boolean :default true))
  (`|ExecutionSequence`
    (:`then_0`
      (bind _valid_ (`self.CheckIfContainsEveryKey` (`self.Speeds`) "Speeds"))
      (if (not _valid_)
        (set `local.(Local) Success?` false)))
    (:`then_1`
      (bind _valid__2 (`self.CheckIfContainsEveryKey` (`self.IncreaseSpeedMultipliers`) "IncreseSpeedMultipliers"))
      (if (not _valid__2)
        (set `local.(Local) Success?` false)))
    (:`then_2`
      (bind _valid__3 (`self.CheckIfContainsEveryKey` (`self.DecreaseSpeedMultipliers`) "IncreseSpeedMultipliers"))
      (if (not _valid__3)
        (set `local.(Local) Success?` false)))
    (:`then_3`
      (return (`local.(Local) Success?`)))))

(fn `DebugVariables`
  (params (Debug :type Boolean))
  (if Debug
    (`self.Debug_Variable` "MaxWalkSpeed: " (`KismetStringLibrary.Conv_Int64ToString` (`KismetMathLibrary.Conv_DoubleToInt64` (`CharacterMovementComponent.MaxWalkSpeed` (`self.CharacterMovementRef`)))) true true false true 0.0 (struct :`G` 0.616667 :`B` 0.070607 :`A` 1.0))
    (`self.Debug_Reference` "CharacterRef: " (`self.CharacterRef`) true true false true 0.0 (struct :`G` 0.617207 :`B` 0.07036 :`A` 1.0))
    (`self.Debug_Reference` "DebugBool: " (`self.CharacterMovementRef`) true true false true 0.0 (struct :`G` 0.617207 :`B` 0.07036 :`A` 1.0))
    (`self.Debug_Variable` "DefaultCapsuleHalfHeight: " (`KismetStringLibrary.Conv_DoubleToString` (`self.DefaultCapsuleHalfHeight`)) true true false true 0.0 (struct :`G` 0.616667 :`B` 0.070607 :`A` 1.0))
    (`self.Debug_Variable` "RunningState: " (`|GetEnumeratorNameAsString` (`self.RunningState`)) true true false true 0.0 (struct :`G` 0.616667 :`B` 0.070607 :`A` 1.0))
    (`self.Debug_Variable` "bSprintKeyDown: " (`KismetStringLibrary.Conv_BoolToString` (`self.bSprintKeyDown`)) true true false true 0.0 (struct :`G` 0.616667 :`B` 0.070607 :`A` 1.0))
    (`self.Debug_Variable` "bMoving: " (`KismetStringLibrary.Conv_BoolToString` (`self.bMoving`)) true true false true 0.0 (struct :`G` 0.616667 :`B` 0.070607 :`A` 1.0))
    (`self.Debug_Reference` "AimingComponentRef: " (`self.AimingComponentRef`) true true false true 0.0 (struct :`G` 0.617207 :`B` 0.07036 :`A` 1.0))
    (`self.Debug_Reference` "ParticleEmiterRef: " (`self.ParticleEmiterRef`) true true false true 0.0 (struct :`G` 0.617207 :`B` 0.07036 :`A` 1.0))
    (return)
    (else
      (return))))

(fn `FindNewRunningState`
  (returns (NewRunningState :type "/Game/MovementMechanics/DynamicRunning/ERunningState Enum"))
  (locals (`(local) RunningState` :type "/Game/MovementMechanics/DynamicRunning/ERunningState Enum"))
  (`|ExecutionSequence`
    (:`then_0`
      (if (`NavMovementComponent.IsMovingOnGround` (`self.CharacterMovementRef`))
        (if (== (`CapsuleComponent.CapsuleHalfHeight` (`Character.CapsuleComponent` (`self.CharacterRef`))) (`self.DefaultCapsuleHalfHeight`))
          (if (`self.bMoving`)
            (if (`self.bSprintKeyDown`)
              (set `local.(local) RunningState` "NewEnumerator3")
              (else
                (set `local.(local) RunningState` "NewEnumerator2")))
            (else
              (set `local.(local) RunningState` "NewEnumerator1")))
          (else
            (set `local.(local) RunningState` "NewEnumerator0")))
        (else
          (set `local.(local) RunningState` "NewEnumerator4"))))
    (:`then_1`
      (return (`local.(local) RunningState`)))))

(fn `IsOwnerMoving`
  (params (AxisValue :type "Float (double-precision)"))
  (returns (`IsMoving?` :type Boolean))
  (return (and (> AxisValue 0.0) (> (`KismetMathLibrary.VSize` (`MovementComponent.Velocity` (`self.CharacterMovementRef`))) (`self.MinDisperseSpeed`)))))

(fn `OnRep_AimingComponentRef`
  (`self.SpawnNiagaraEmiter`)
  (return))

(fn `ResolveEmiterVisibility`
  (returns (`Valid?` :type Boolean) (`IsEmiterVisible?` :type Boolean))
  (bind _value (`BlueprintMapLibrary.Map_Find` (`self.StatesEmitingParticles`) (`self.RunningState`)))
  (bind _particleemiterref (`self.ParticleEmiterRef`)
    (:`then`
      (`SceneComponent.SetVisibility` _particleemiterref _value true)
      (return true _value))
    (:`else`
      (return false false))))

(fn `Set_AimingComponentRef`
  (params (AimingComponentRef :type "SceneComponent Object Reference"))
  (returns (`Success?` :type Boolean))
  (`self.AimingComponentRef`
    (:`then`
      (return false))
    (:`else`
      (set `self.AimingComponentRef` AimingComponentRef)
      (return true))))

(fn `Set_OwningCharacter`
  (params (CharacterRef :type "Actor Object Reference"))
  (returns (`Success?` :type Boolean))
  (bind _ascharacter (cast `Character` CharacterRef)
    (:`then`
      (bind _output_get (set `self.CharacterRef` _ascharacter))
      (set `self.CharacterMovementRef` (`Character.CharacterMovement` _output_get))
      (set `self.DefaultCapsuleHalfHeight` (`CapsuleComponent.CapsuleHalfHeight` (`Character.CapsuleComponent` _output_get)))
      (return true))
    (:`CastFailed`
      (`self.Throw_CastFailedError` "Character" CharacterRef)
      (return false))))

(fn `SpawnNiagaraEmiter`
  (returns (`Success?` :type Boolean))
  (bind _aimingcomponentref (`self.AimingComponentRef`)
    (:`then`
      (bind _returnvalue (`NiagaraFunctionLibrary.SpawnSystemAttached` (`self.NiagaraParticleSystem`) _aimingcomponentref "None" (.location (`self.ParticleEmiterOffset`)) (.rotation (`self.ParticleEmiterOffset`)) "KeepRelativeOffset"))
      (set `self.ParticleEmiterRef` _returnvalue)
      (return true))
    (:`else`
      (return false))))

(fn `Tick_FindNewWalkSpeed`
  (params (DeltaSeconds :type "Float (single-precision)"))
  (returns (`New Walk Speed` :type "Float (single-precision)"))
  (if (> (`CharacterMovementComponent.MaxWalkSpeed` (`self.CharacterMovementRef`)) (`BlueprintMapLibrary.Map_Find` (`self.Speeds`) (`self.RunningState`)))
    (return (- (`CharacterMovementComponent.MaxWalkSpeed` (`self.CharacterMovementRef`)) (* (`BlueprintMapLibrary.Map_Find` (`self.DecreaseSpeedMultipliers`) (`self.RunningState`)) (`local.DeltaSeconds`))))
    (else
      (return (+ (`CharacterMovementComponent.MaxWalkSpeed` (`self.CharacterMovementRef`)) (* (`BlueprintMapLibrary.Map_Find` (`self.IncreaseSpeedMultipliers`) (`self.RunningState`)) (`local.DeltaSeconds`)))))))