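; Character component that adds crouching, sprinting and sliding through a movement state machine driven by crouch and sprint input.
; Tick blends capsule height and aiming component offset, and leaves crouch once an overhead trace allows standing.
; Crouching from sprint starts a slide with zero ground friction and a slope-based force applied on a one-second cooldown.
; The slide has no exit yet (marked FIXME), and debug printing runs every tick.
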(event `self.ReceiveBeginPlay`
  (`self.FindOwningCharacter`)
  (`self.FindDefaultValiues`))

(event `self.ReceiveTick`
  (params (DeltaSeconds :type "Float (single-precision)"))
  ;[1 1 1] Tick
  (`|ExecutionSequence`
    (:`then_0`
      (`self.Tick_CrouchingProgress` DeltaSeconds))
    (:`then_1`
      (`self.Switch On MovementState`
        (:`Crouching`
          (if (`self.CanStand`)
            (`self.Set_CrouchingState` (`self.FindNewCrouchingState`))))
        (:`Sliding`
          (`self.Cooldown` 1.0
            (:`execute `
              (`self.Tick_Slide`))))))
    (:`then_2`
      (`self.Debug_PrintVariables` true))))

(event `SprintKeyDown`
  ;[1 1 1] Input Logic
  (set `self.bSprintKeyDown` true)
  (`self.Switch On MovementState`
    (:`Walking`
      (`self.Set_CrouchingState` "NewEnumerator1" :!label _label))
    (:`Crouching`
      (if (`self.CanStand`)
        (goto _label)))))

(event `SprintKeyUp`
  ;[1 1 1] Input Logic
  (set `self.bSprintKeyDown` false)
  (`self.Switch On MovementState`))

(event `CrouchKeyDown`
  ;[1 1 1] Input Logic
  (set `self.bCrouchKeyDown` true)
  (`self.Switch On MovementState`
    (:`Walking`
      (`self.Set_CrouchingState` "NewEnumerator2"))
    (:`Sprinting`
      (`self.Set_CrouchingState` "NewEnumerator3"))))

(event `CrouchKeyUp`
  ;[1 1 1] Input Logic
  (set `self.bCrouchKeyDown` false))

(fn `CalculateFloorInfluence`
  (params (FloorNormal :type "Vector Structure"))
  (returns (ReturnValue :type "Vector Structure"))
  (if (== FloorNormal (`KismetMathLibrary.Vector_Up`))
    (return (0.0 0.0 0.0))
    (else
      (return (`KismetMathLibrary.Normal` (`KismetMathLibrary.Cross_VectorVector` FloorNormal (`KismetMathLibrary.Cross_VectorVector` FloorNormal (`KismetMathLibrary.Vector_Up`))))))))

(fn `CanSprint`
  (returns (Result :type Boolean))
  (if (`self.bSprintKeyDown`)
    (return (and (`self.CanStand`) (not (`NavMovementComponent.IsFalling` (`self.CharacterMovementRef`)))))
    (else
      (return false))))

(fn `CanStand`
  (returns (Result :type Boolean))
  (bind _returnvalue (- (`Actor.K2_GetActorLocation` (`self.CharacterRef`)) (`KismetMathLibrary.MakeVector` 0.0 0.0 (`CapsuleComponent.GetScaledCapsuleHalfHeight` (`self.CapsuleComponentRef`)))))
  (if (`self.bCrouchKeyDown`)
    (return false)
    (else
      (bind (_outhit _returnvalue_2) (`KismetSystemLibrary.LineTraceSingle` _returnvalue (+ _returnvalue (`KismetMathLibrary.MakeVector` 0.0 0.0 (* (`self.DefaultStandingCapsuleHalfHeight`) 2.0))) "TraceTypeQuery1" false (`|MakeArray` (`self.CharacterRef`) :!type "Actor Object Reference")))
      (return (not _returnvalue_2)))))

(fn `Debug_PrintVariables`
  (params (Debug :type Boolean :default true))
  (if Debug
    (`self.Debug_Reference` "CharacterRef: " (`self.CharacterRef`) true true false true 0.0 (struct :`R` 0.754003 :`G` 0.879167 :`A` 1.0))
    (`self.Debug_Reference` "CharacterMovementRef: " (`self.CharacterMovementRef`) true true false true 0.0 (struct :`R` 0.754003 :`G` 0.879167 :`A` 1.0))
    (`self.Debug_Reference` "CapsuleComponentRef: " (`self.CapsuleComponentRef`) true true false true 0.0 (struct :`R` 0.754003 :`G` 0.879167 :`A` 1.0))
    (`self.Debug_Reference` "AimingComponentRef: " (`self.AimingComponentRef`) true true false true 0.0 (struct :`R` 0.754003 :`G` 0.879167 :`A` 1.0))
    (`self.Debug_Variable` "DefaultStandingCapsuleHalfHeight: " (`KismetStringLibrary.Conv_DoubleToString` (`self.DefaultStandingCapsuleHalfHeight`)) true true false true 0.0 (struct :`R` 0.752942 :`G` 0.879622 :`A` 1.0))
    (`self.Debug_Variable` "DefaultCameraZOffset: " (`KismetStringLibrary.Conv_DoubleToString` (`self.DefaultCameraZOffset`)) true true false true 0.0 (struct :`R` 0.752942 :`G` 0.879622 :`A` 1.0))
    (`self.Debug_Variable` "DefaultGroundFriction: " (`KismetStringLibrary.Conv_DoubleToString` (`self.DefaultGroundFriction`)) true true false true 0.0 (struct :`R` 0.752942 :`G` 0.879622 :`A` 1.0))
    (`self.Debug_Variable` "DefaultBrakingDecelerationWalking: " (`KismetStringLibrary.Conv_DoubleToString` (`self.DefaultBrakingDecelerationWalking`)) true true false true 0.0 (struct :`R` 0.752942 :`G` 0.879622 :`A` 1.0))
    (`self.Debug_Variable` "MovementState: " (`|GetEnumeratorNameAsString` (`self.MovementState`)) true true false true 0.0 (struct :`R` 0.752942 :`G` 0.879622 :`A` 1.0))
    (`self.Debug_Variable` "bSprintKeyDown: " (`KismetStringLibrary.Conv_BoolToString` (`self.bSprintKeyDown`)) true true false true 0.0 (struct :`R` 0.752942 :`G` 0.879622 :`A` 1.0))
    (`self.Debug_Variable` "bCrouchKeyDown: " (`KismetStringLibrary.Conv_BoolToString` (`self.bCrouchKeyDown`)) true true false true 0.0 (struct :`R` 0.752942 :`G` 0.879622 :`A` 1.0))
    (`self.Debug_Variable` "StandingProgress: " (`KismetStringLibrary.Conv_DoubleToString` (`self.StandingProgress`)) true true false true 0.0 (struct :`R` 0.752942 :`G` 0.879622 :`A` 1.0))
    (else
      (return))))

(fn `Event_OnLanded`
  (params (Hit :type "HitResult Structure"))
  (returns (`Valid?` :type Boolean) (`Success?` :type Boolean))
  (return false false))

(fn `FindDefaultValiues`
  (bind _charactermovementref (`self.CharacterMovementRef`))
  (set `self.DefaultStandingCapsuleHalfHeight` (`CapsuleComponent.GetScaledCapsuleHalfHeight` (`self.CapsuleComponentRef`)))
  (set `self.DefaultGroundFriction` (`CharacterMovementComponent.GroundFriction` _charactermovementref))
  (set `self.DefaultBrakingDecelerationWalking` (`CharacterMovementComponent.BrakingDecelerationWalking` _charactermovementref))
  (return))

(fn `FindNewCrouchingState`
  (returns (NewCrouchingState :type "/Game/MovementMechanics/CrouchingAndSliding/ECrouchingState Enum"))
  (return (select `bool` (`self.CanSprint`) :`false` (select `bool` (`self.CanStand`) :`false` "NewEnumerator2" :`true` "NewEnumerator0" :!type "/Game/MovementMechanics/CrouchingAndSliding/ECrouchingState Enum") :`true` "NewEnumerator1")))

(fn `FindOwningCharacter`
  (returns (`Success?` :type Boolean))
  (bind _ascharacter (cast `Character` (`self.GetOwner`))
    (:`then`
      (bind _output_get (set `self.CharacterRef` _ascharacter))
      (set `self.CharacterMovementRef` (`Character.CharacterMovement` _output_get))
      (set `self.CapsuleComponentRef` (`Character.CapsuleComponent` _output_get))
      (return true))
    (:`CastFailed`
      (`KismetSystemLibrary.PrintString` "Component_PhysicBaseSliding: Cast to ThirdPersonCharacter failed" true true (struct :`R` 1.0 :`B` 0.014055 :`A` 1.0))
      (return false))))

(fn `Get_CrouchingState`
  (returns (CrouchingState :type "/Game/MovementMechanics/CrouchingAndSliding/ECrouchingState Enum"))
  (return (`self.MovementState`)))

(fn `Input_Action0_KeyDown`
  (returns (`Valid?` :type Boolean) (`Success?` :type Boolean))
  (return false false))

(fn `Input_Action0_KeyUp`
  (returns (`Valid?` :type Boolean) (`Success?` :type Boolean))
  (return false false))

(fn `Input_Axis_MoveForward`
  (params (AxisValue :type "Float (double-precision)"))
  (returns (`Valid?` :type Boolean) (`Success?` :type Boolean))
  (return false false))

(fn `Input_Axis_MoveRight`
  (params (AxisValue :type "Float (double-precision)"))
  (returns (`Valid?` :type Boolean) (`Success?` :type Boolean))
  (return false false))

(fn `Input_Crouch_KeyDown`
  (returns (`Valid?` :type Boolean) (`Success?` :type Boolean))
  (`self.CrouchKeyDown`)
  (return true true))

(fn `Input_Crouch_KeyUp`
  (returns (`Valid?` :type Boolean) (`Success?` :type Boolean))
  (`self.CrouchKeyUp`)
  (return true true))

(fn `Input_Debug_KeyDown`
  (returns (`Valid?` :type Boolean) (`Success?` :type Boolean))
  (return false false))

(fn `Input_Debug_KeyUp`
  (returns (`Valid?` :type Boolean) (`Success?` :type Boolean))
  (return false false))

(fn `Input_Jump_KeyDown`
  (returns (`Valid?` :type Boolean) (`Success?` :type Boolean))
  (return false false))

(fn `Input_Jump_KeyUp`
  (returns (`Valid?` :type Boolean) (`Success?` :type Boolean))
  (return false false))

(fn `Input_Sprint_KeyDown`
  (returns (`Valid?` :type Boolean) (`Success?` :type Boolean))
  (`self.SprintKeyDown`)
  (return true true))

(fn `Input_Sprint_KeyUp`
  (returns (`Valid?` :type Boolean) (`Success?` :type Boolean))
  (`self.SprintKeyUp`)
  (return true true))

(fn `OnMovementStateChange`
  (params (PrevMovementState :type "/Game/MovementMechanics/CrouchingAndSliding/ECrouchingState Enum" :default "NewEnumerator0"))
  (bind _charactermovementref (`self.CharacterMovementRef`))
  (bind _charactermovementref_2 (`self.CharacterMovementRef`))
  (`|ExecutionSequence`
    (:`then_0`
      (switch `/Game/MovementMechanics/CrouchingAndSliding/ECrouchingState` (`local.PrevMovementState`)
        (:`NewEnumerator3`
          (set `CharacterMovementComponent.GroundFriction` (`self.DefaultGroundFriction`) _charactermovementref_2)
          (set `CharacterMovementComponent.BrakingDecelerationWalking` (`self.DefaultBrakingDecelerationWalking`) _charactermovementref_2))))
    (:`then_1`
      (`self.Switch On MovementState`
        (:`Sliding`
          (set `MovementComponent.Velocity` (* (`Actor.GetActorForwardVector` (`self.CharacterRef`)) (`CharacterMovementComponent.MaxWalkSpeed` (`self.CharacterMovementRef`))) _charactermovementref)
          (set `CharacterMovementComponent.GroundFriction` 0.0 _charactermovementref)
          (set `CharacterMovementComponent.BrakingDecelerationWalking` 700.0 _charactermovementref))))
    (:`then_2`
      (return))))

(fn `Set_AimingComponentRef`
  (params (AimingComponentRef :type "SceneComponent Object Reference"))
  (returns (`Success?` :type Boolean))
  (bind _relativelocation_x (`KismetMathLibrary.BreakVector` (`SceneComponent.RelativeLocation` (`self.AimingComponentRef`))))
  (`self.AimingComponentRef`
    (:`then`
      (return false))
    (:`else`
      (set `self.AimingComponentRef` AimingComponentRef)
      (set `self.DefaultCameraZOffset` _relativelocation_x)
      (return true))))

(fn `Set_CrouchingState`
  (params (CrouchingState :type "/Game/MovementMechanics/CrouchingAndSliding/ECrouchingState Enum" :default "NewEnumerator0"))
  (returns (`HasMovementStateChanged?` :type Boolean))
  (locals (`PrevMovementState (Local)` :type "/Game/MovementMechanics/CrouchingAndSliding/ECrouchingState Enum"))
  (if (`|EnumInequality` CrouchingState (`self.MovementState`))
    (bind _output_get (set `local.PrevMovementState (Local)` (`self.MovementState`)))
    (set `self.MovementState` CrouchingState)
    (`self.OnMovementStateChange` _output_get)
    (return true)
    (else
      (return false))))

(fn `Tick_ChangeCapsuleHeight`
  (params (Progress :type "Float (double-precision)"))
  (bind _aimingcomponentref (`self.AimingComponentRef`))
  (bind (_relativelocation_x _relativelocation_y _relativelocation_z) (`KismetMathLibrary.BreakVector` (`SceneComponent.RelativeLocation` _aimingcomponentref)))
  (`CapsuleComponent.SetCapsuleHalfHeight` (`self.CapsuleComponentRef`) (`KismetMathLibrary.MapRangeClamped` Progress 0.0 1.0 0.35 (`self.DefaultStandingCapsuleHalfHeight`)) true)
  (`SceneComponent.K2_SetRelativeLocation` _aimingcomponentref (`KismetMathLibrary.MakeVector` (`KismetMathLibrary.MapRangeClamped` Progress 0.0 1.0 -30.0 (`self.DefaultCameraZOffset`)) _relativelocation_y _relativelocation_z) false false)
  (return))

(fn `Tick_CrouchingProgress`
  (params (DeltaSeconds :type "Float (double-precision)") (ProgressChangePerSecond :type "Float (double-precision)" :default 2.5))
  (`self.Switch On MovementState`
    (:`Walking`
      (if (< (`self.StandingProgress`) 1.0) :!label _label
        (bind _output_get (set `self.StandingProgress` (+ (`self.StandingProgress`) (* (`local.DeltaSeconds`) (`local.ProgressChangePerSecond`)))))
        (`self.Tick_ChangeCapsuleHeight` _output_get)
        (return)))
    (:`Sprinting`
      (goto _label))
    (:`Crouching`
      (if (> (`self.StandingProgress`) 0.0) :!label _label_2
        (bind _output_get_2 (set `self.StandingProgress` (- (`self.StandingProgress`) (* (`local.DeltaSeconds`) (`local.ProgressChangePerSecond`)))))
        (`self.Tick_ChangeCapsuleHeight` _output_get_2)
        (return)))
    (:`Sliding`
      (goto _label_2))))

(fn `Tick_Slide`
  (bind _charactermovementref (`self.CharacterMovementRef`))
  (bind _charactermovementref_2 (`self.CharacterMovementRef`))
  (bind (_currentfloor_bblockinghit _currentfloor_bwalkablefloor _currentfloor_blinetrace _currentfloor_floordist _currentfloor_linedist _currentfloor_hitresult) (break `FindFloorResult` (`CharacterMovementComponent.CurrentFloor` _charactermovementref_2)))
  (`|ExecutionSequence`
    (:`then_0`
      (`CharacterMovementComponent.AddForce` (`self.CharacterMovementRef`) (* (`self.CalculateFloorInfluence` (`.Normal` (`GameplayStatics.BreakHitResult` _currentfloor_hitresult))) (* (`CharacterMovementComponent.MaxWalkSpeed` _charactermovementref_2) 400.0))))
    (:`then_1`
      (if (> (`KismetMathLibrary.VSize` (`Actor.GetVelocity` (`self.CharacterRef`))) 0.0)
        (set `MovementComponent.Velocity` (* (`KismetMathLibrary.Normal` (`Actor.GetVelocity` (`self.CharacterRef`))) (`CharacterMovementComponent.MaxWalkSpeed` _charactermovementref)) _charactermovementref)))
    (:`then_2`
      ;[1 0 0] FIXME tutaj czegos brakuje
      (if (< (`KismetMathLibrary.VSize` (`Actor.GetVelocity` (`self.CharacterRef`))) (`CharacterMovementComponent.MaxWalkSpeed` (`self.CharacterMovementRef`)))
        _))
    (:`then_3`
      (return))))