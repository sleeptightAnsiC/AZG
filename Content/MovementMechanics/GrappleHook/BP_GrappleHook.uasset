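; BP_GrappleHook is the projectile actor for the grapple hook movement mechanic, covering only the hook's flight and range limit.
; On BeginPlay it passes its Velocity and gravity scale variables to the ProjectileMovement component and records its start location.
; Each Tick it measures straight-line distance from that start and destroys itself beyond MaxDistance.
; This Blueprint's graphs contain no hit, attach or pull logic.
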(event `self.ReceiveBeginPlay`
  (set `MovementComponent.Velocity` (`self.Velocity`) (`self.ProjectileMovement`))
  (set `ProjectileMovementComponent.ProjectileGravityScale` (`self.ProjectileGravityScale`) (`self.ProjectileMovement`))
  (set `self.StartLocation` (`self.K2_GetActorLocation`)))

(event `self.ReceiveTick`
  (params (DeltaSeconds :type "Float (single-precision)"))
  (if (> (`KismetMathLibrary.Vector_Distance` (`self.StartLocation`) (`self.K2_GetActorLocation`)) (`self.MaxDistance`))
    (`self.K2_DestroyActor` self)))

(fn `UserConstructionScript`)