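; Grapple hook component for a Character that fires a projectile and cable at a line-traced aim point.
; A state enum routes Fire1 (fire, pull, cancel), Jump (release) and Tick, following ground/air changes once attached.
; Tick applies pulling force or a dot-product rope force for swinging, and breaks the hook on distance or position checks.
; Swinging overrides friction, gravity and air control, restored when the projectile's OnDestroyed handler resets everything.
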(event `self.ReceiveBeginPlay`
  (bind _output_get (set `self.OwningActorRef` (`self.GetOwner`)))
  (bind _ascharacter (cast `Character` _output_get))
  (`self.Set_OwningCharacter` _ascharacter))

(event `InputAction|Fire1` :consume false :overrideparent false
  (params (Key :type "Key Structure"))
  (:`Pressed`
    (`self.SwitchOnGrappleState`
      (:`ReadyToFire`
        ;[1 1 1] Fire Grapple
        (set `self.GrappleState` "NewEnumerator1")
        (bind _result (`self.FindGrappleHitLocation` 1500.0 (`self.bDebugMode`)))
        (bind (_grappleprojectileref _grapplecableref) (`self.Fire Grapple` _result))
        (set `self.GrappleCableRef` _grapplecableref)
        (bind _output_get (set `self.GrappleProjectileRef` _grappleprojectileref))
        (`self.BindTheGrappleFunctions` _output_get))
      (:`Firing`
        (`self.DestroyGrappleHook` :!label _label))
      (:`AttachedToTarget - OnGround`
        (`self.FindPoolingDirection2D` :!label _label_2)
        (set `self.GrappleState` "NewEnumerator4"))
      (:`AttachedToTarget - InAir`
        (goto _label_2))
      (:`AttachedToTarget - Pulling`
        (goto _label)))))

(event `InputAction|Jump` :consume false :overrideparent false
  (params (Key :type "Key Structure"))
  (:`Pressed`
    (`self.SwitchOnGrappleState`
      (:`AttachedToTarget - InAir`
        _)
      (:`AttachedToTarget - Pulling`
        _))
    (`self.DestroyGrappleHook`)))

(event `self.ReceiveTick`
  (params (DeltaSeconds :type "Float (single-precision)"))
  (`|ExecutionSequence`
    (:`then_0`
      (`self.Tick_CheckIfOnGroundOrInAir` true))
    (:`then_1`
      (`self.SwitchOnGrappleState`
        (:`AttachedToTarget - OnGround`
          (if (`self.bGrappleSwinging`)
            (`self.Tick_AddSwingingForce` DeltaSeconds))
          (`self.DestroyGrappleHookOnGivenConditions` false 250.0 false false 300.0 true 1000.0))
        (:`AttachedToTarget - InAir`
          (`self.Tick_AddSwingingForce` DeltaSeconds)
          (`self.DestroyGrappleHookOnGivenConditions` false 250.0 false false 300.0 true 1100.0))
        (:`AttachedToTarget - Pulling`
          ;[1 1 1] Pulling towards grapple hit location
          (`self.Tick_AddPullingForce` 500000.0)
          (`self.DestroyGrappleHookOnGivenConditions` true))))
    (:`then_2`
      ;[1 1 1] Debug
      (`self.Tick_DebugVariables` (`self.bDebugMode`)))))

(fn `BindTheGrappleFunctions`
  (params (GrappleHookRef :type "/Game/MovementMechanics/GrappleHook/BP_GrappleProjectile Object Reference"))
  (add `Actor.OnActorHit` GrappleHookRef (`|CreateDelegate` :!event `OnGrappleHit`))
  (add `Actor.OnDestroyed` GrappleHookRef (`|CreateDelegate` :!event `OnGrappleHookDestroyed`))
  (return))

(fn `DestroyGrappleHook`
  (returns (`Success?` :type Boolean))
  (bind _grappleprojectileref (`self.GrappleProjectileRef`)
    (:`then`
      (`Actor.K2_DestroyActor` _grappleprojectileref)
      (return true))
    (:`else`
      (return true))))

(fn `DestroyGrappleHookOnGivenConditions`
  (params (ByBeingTooCloseToGrappleHitPoint :type Boolean :default true) (MinDistance :type "Float (double-precision)" :default 250.0) (ByBeingFutherThanGrappleHitPoint :type Boolean :default true) (ByBeingHigherThanGrappleHitPoint :type Boolean :default true) (HowHigherCanBe :type "Float (double-precision)" :default 300.0) (ByBeingTooFarToGrappleHitPoint :type Boolean) (MaxDistance :type "Float (double-precision)" :default 2000.0))
  (returns (`DidDestroyGrappleHook?` :type Boolean))
  (bind (_returnvalue_x _returnvalue_y _returnvalue_z) (`KismetMathLibrary.BreakVector` (`SceneComponent.K2_GetComponentLocation` (`self.SelectBetween_OwningActor&AimingComponent`))))
  (`|ExecutionSequence`
    (:`then_0`
      (if (and (`local.ByBeingTooCloseToGrappleHitPoint`) (< (`.Distance` (`self.Get_DistanceToGrappleProjectile`)) (`local.MinDistance`)))
        (bind _success_ (`self.DestroyGrappleHook`))
        (return _success_)))
    (:`then_1`
      (if (and (`local.ByBeingTooFarToGrappleHitPoint`) (> (`.Distance` (`self.Get_DistanceToGrappleProjectile`)) (`local.MaxDistance`)))
        (bind _success__2 (`self.DestroyGrappleHook`))
        (return _success__2)))
    (:`then_2`
      (if (and (`local.ByBeingFutherThanGrappleHitPoint`) (not (`self.IsInFrontOfPoolingDirection?`)))
        (bind _success__3 (`self.DestroyGrappleHook`))
        (return _success__3)))
    (:`then_3`
      (if (and (`local.ByBeingHigherThanGrappleHitPoint`) (> _returnvalue_z (+ (.z (.location (`.Result` (`self.Get_GrappleProjectileTransform`)))) (`local.HowHigherCanBe`))))
        (bind _success__4 (`self.DestroyGrappleHook`))
        (return _success__4)))
    (:`then_4`
      (return false))))

(fn `FindGrappleHitLocation`
  (params (Distance :type "Float (double-precision)" :default 1500.0) (DrawDebug :type Boolean))
  (returns (Result :type "Vector Structure"))
  (bind _result (`self.SelectBetween_OwningActor&AimingComponent`))
  (bind _returnvalue (`SceneComponent.K2_GetComponentLocation` _result))
  (bind (_outhit _returnvalue_2) (`KismetSystemLibrary.LineTraceSingle` _returnvalue (+ _returnvalue (* (`SceneComponent.GetForwardVector` _result) (`local.Distance`))) "TraceTypeQuery1" false (`|MakeArray` (`self.OwningActorRef`)) (select `bool` (`local.DrawDebug`) :`true` "ForDuration" :!type "EDrawDebugTrace Enum") true (struct :`G` 0.068478 :`B` 0.313989 :`A` 1.0)))
  (bind (_bblockinghit _binitialoverlap _time _distance _location _impactpoint _normal _impactnormal _physmat _hitactor _hitcomponent _hitbonename _bonename _hititem _elementindex _faceindex _tracestart _traceend) (`GameplayStatics.BreakHitResult` _outhit))
  (return (select `bool` _returnvalue_2 :`false` _traceend :`true` _location)))

(fn `FindPoolingDirection2D`
  (returns (`Valid?` :type Boolean))
  (bind (_direction3d _valid_ _direction2d) (`self.Get_DirectionToGrappleProjectile`))
  (set `self.PoolingDirection2D` _direction2d)
  (return _valid_))

(fn `Fire Grapple`
  (params (TargetLocation :type "Vector Structure") (LocalOffset :type "Vector Structure" :default (-30.0 -30.0 50.0)) (GravityScale :type "Float (double-precision)") (Speed :type "Float (double-precision)" :default 5000.0) (MaxDistance :type "Float (double-precision)" :default 1500.0))
  (returns (GrappleProjectileRef :type "/Game/MovementMechanics/GrappleHook/BP_GrappleProjectile Object Reference") (GrappleCableRef :type "CableActor Object Reference"))
  (locals (`FireDirection (local)` :type "Vector Structure" :default (0.0 0.0 0.0)) (`GrappleProjectileRef (local)` :type "/Game/MovementMechanics/GrappleHook/BP_GrappleProjectile Object Reference") (`GrappleCableRef (local)` :type "CableActor Object Reference"))
  (bind _grappleprojectileref__local_ (`local.GrappleProjectileRef (local)`))
  (set `local.FireDirection (local)` (`KismetMathLibrary.Normal` (- (`local.TargetLocation`) (`self.CableStartLocation` (`local.LocalOffset`)))))
  (bind _returnvalue (`|SpawnActorFromClass` "/Game/MovementMechanics/GrappleHook/BP_GrappleProjectile.BP_GrappleProjectile_C" (`KismetMathLibrary.MakeTransform` (`self.CableStartLocation` (`local.LocalOffset`))) "Undefined" "OverrideRootScale" (`self.OwningActorRef`) (* (`local.FireDirection (local)`) (`local.Speed`)) (`local.GravityScale`) (`local.MaxDistance`) null))
  (set `local.GrappleProjectileRef (local)` _returnvalue)
  (bind _returnvalue_2 (`|SpawnActorFromClass` "/Game/MovementMechanics/GrappleHook/BP_GrappleCable.BP_GrappleCable_C" (`KismetMathLibrary.MakeTransform` (`self.CableStartLocation` (`local.LocalOffset`)) (`KismetMathLibrary.MakeRotFromX` (`local.FireDirection (local)`))) "Undefined" "OverrideRootScale" (`self.OwningActorRef`) null))
  (set `local.GrappleCableRef (local)` _returnvalue_2)
  ;[1 1 1] Chwilowy fix przez buga ze znikającą liną
  (`CableComponent.SetAttachEndTo` (`CableActor.CableComponent` (`local.GrappleCableRef (local)`)) (`self.OwningActorRef`) "None" "None")
  (`Actor.K2_AttachToActor` (`local.GrappleCableRef (local)`) (`local.GrappleProjectileRef (local)`) "None" "KeepWorld" "KeepWorld" "KeepWorld" true)
  (`GameplayStatics.PlaySoundAtLocation` (`self.Sound_OnGrappleHookFired`) (`Actor.K2_GetActorLocation` _grappleprojectileref__local_) (struct) 1.0 1.0 0.0 null null null null)
  (return _grappleprojectileref__local_ (`local.GrappleCableRef (local)`)))

(fn `Get_DirectionToGrappleProjectile`
  (returns (Direction3D :type "Vector Structure") (`Valid?` :type Boolean) (Direction2D :type "Vector Structure"))
  (bind _grappleprojectileref (`self.GrappleProjectileRef`)
    (:`then`
      (bind _returnvalue (`KismetMathLibrary.Normal` (- (`Actor.K2_GetActorLocation` _grappleprojectileref) (`SceneComponent.K2_GetComponentLocation` (`self.SelectBetween_OwningActor&AimingComponent`)))))
      (return _returnvalue true (`KismetMathLibrary.Normal` (`KismetMathLibrary.MakeVector` (.x _returnvalue) (.y _returnvalue)))))
    (:`else`
      (return (0.0 0.0 0.0) false (0.0 0.0 0.0)))))

(fn `Get_DistanceToGrappleProjectile`
  (returns (`Valid?` :type Boolean) (Distance :type "Float (double-precision)"))
  (bind _grappleprojectileref (`self.GrappleProjectileRef`)
    (:`then`
      (return true (`KismetMathLibrary.Vector_Distance` (`Actor.K2_GetActorLocation` _grappleprojectileref) (`SceneComponent.K2_GetComponentLocation` (`self.SelectBetween_OwningActor&AimingComponent`)))))
    (:`else`
      (return false 0.0))))

(fn `Get_GrappleProjectileTransform`
  (returns (`Valid?` :type Boolean) (Result :type "Transform Structure"))
  (bind _grappleprojectileref (`self.GrappleProjectileRef`)
    (:`then`
      (return (select `/Game/MovementMechanics/GrappleHook/Enum_GrappleState` (`self.GrappleState`) :`NewEnumerator2` true) (`Actor.GetTransform` _grappleprojectileref)))
    (:`else`
      (return false (`KismetMathLibrary.MakeTransform` (0.0 0.0 0.0) (struct) (0.0 0.0 0.0))))))

(fn `Get_HorizontalDistanceToGrappleProjectile`
  (returns (ReturnValue :type "Float (single-precision)") (`Valid?` :type Boolean))
  (bind _grappleprojectileref (`self.GrappleProjectileRef`)
    (:`then`
      (return (`Actor.GetHorizontalDistanceTo` _grappleprojectileref (`self.OwningActorRef`)) true))
    (:`else`
      (return 0.0 false))))

(fn `Get_VerticalDistanceToGrappleProjectile`
  (returns (ReturnValue :type "Float (single-precision)") (`Success?` :type Boolean))
  (bind _grappleprojectileref (`self.GrappleProjectileRef`)
    (:`then`
      (return (`Actor.GetVerticalDistanceTo` _grappleprojectileref (`self.OwningActorRef`)) true))
    (:`else`
      (return 0.0 false))))

(fn `IsGrappleInUse?`
  (returns (Result :type Boolean))
  (return (select `/Game/MovementMechanics/GrappleHook/Enum_GrappleState` (`self.GrappleState`) :`NewEnumerator1` true :`NewEnumerator2` true :`NewEnumerator3` true :`NewEnumerator4` true)))

(fn `IsInFrontOfPoolingDirection?`
  (returns (result :type Boolean) (`Valid?` :type Boolean))
  (bind (_direction3d _valid_ _direction2d) (`self.Get_DirectionToGrappleProjectile`))
  (return (not (< (`KismetMathLibrary.Dot_VectorVector` (`self.PoolingDirection2D`) _direction2d) 0.0)) _valid_))

(fn `OnAirEntered`
  (returns (`success?` :type Boolean))
  (`self.OwningCharacterMovementRef`
    (:`then`
      (set `self.bGrounded` false)
      (if (`|EnumEquality` (`self.GrappleState`) "NewEnumerator2")
        (`self.Set_CharacterSwingingState` true)
        (set `self.GrappleState` "NewEnumerator3")
        (set `self.ImagineryRopeLength` (+ (`.Distance` (`self.Get_DistanceToGrappleProjectile`)) 200.0))
        (return true)))
    (:`else`
      (return false))))

(fn `OnGrappleHit`
  (params (SelfActor :type "Actor Object Reference") (OtherActor :type "Actor Object Reference") (NormalImpulse :type "Vector Structure") (Hit :type "HitResult Structure (by ref)"))
  (if (`self.bGrounded`)
    (set `self.GrappleState` "NewEnumerator2")
    (return)
    (else
      (set `self.GrappleState` "NewEnumerator3")
      (`self.Set_CharacterSwingingState` true)
      (return))))

(fn `OnGrappleHookDestroyed`
  (params (DestroyedActor :type "Actor Object Reference"))
  (`GameplayStatics.PlaySoundAtLocation` (`self.Sound_OnGrappleHookDestroyed`) (`Actor.K2_GetActorLocation` DestroyedActor) (struct) 1.0 1.0 0.0 null null null null)
  (set `self.GrappleProjectileRef` null)
  (set `self.GrappleState` "NewEnumerator0")
  (`self.Set_CharacterSwingingState` false)
  (bind _grapplecableref (`self.GrappleCableRef`)
    (:`then`
      (`Actor.K2_DestroyActor` _grapplecableref)
      (set `self.GrappleCableRef` null)
      (return))
    (:`else`)))

(fn `OnGroundLanded`
  (returns (`Success?` :type Boolean))
  (`self.OwningCharacterMovementRef`
    (:`then`
      (set `self.bGrounded` true)
      (if (`self.bGrappleSwinging`)
        (set `self.ImagineryRopeLength` (+ (`.Distance` (`self.Get_DistanceToGrappleProjectile`)) 200.0))
        (set `self.GrappleState` "NewEnumerator2")
        (return true)))
    (:`else`
      (return false))))

(fn `Set_AimingComponentRef`
  (params (Component :type "SceneComponent Object Reference"))
  (set `self.AimingComponentRef` Component)
  (return))

(fn `Set_CharacterSwingingState`
  (params (`Swinging?` :type Boolean))
  (returns (`Success?` :type Boolean))
  (if `Swinging?`
    (bind _owningcharactermovementref (`self.OwningCharacterMovementRef`)
      (:`then`
        (set `CharacterMovementComponent.GroundFriction` 0.0 _owningcharactermovementref)
        (set `CharacterMovementComponent.GravityScale` 1.8 _owningcharactermovementref)
        (set `CharacterMovementComponent.AirControl` 1.0 _owningcharactermovementref)
        (`CharacterMovementComponent.ClearAccumulatedForces` _owningcharactermovementref)
        (set `self.bGrappleSwinging` true)
        (return true))
      (:`else`
        _))
    (else
      (bind _owningcharactermovementref_2 (`self.OwningCharacterMovementRef`)
        (:`then`
          (set `CharacterMovementComponent.GroundFriction` (`self.DefaultGroundFriction`) _owningcharactermovementref_2)
          (set `CharacterMovementComponent.GravityScale` (`self.DefaultGravityScale`) _owningcharactermovementref_2)
          (set `CharacterMovementComponent.AirControl` (`self.DefaultAirControl`) _owningcharactermovementref_2)
          (set `self.bGrappleSwinging` false)
          (return true))
        (:`else`
          _))))
  (set `self.bGrappleSwinging` false)
  (return false))

(fn `Set_OwningCharacter`
  (params (CharacterRef :type "Character Object Reference"))
  (bind _output_get (set `self.OwningCharacterRef` CharacterRef))
  (bind _output_get_2 (set `self.OwningCharacterMovementRef` (`Character.CharacterMovement` _output_get)))
  (set `self.DefaultGroundFriction` (`CharacterMovementComponent.GroundFriction` _output_get_2))
  (set `self.DefaultGravityScale` (`CharacterMovementComponent.GravityScale` _output_get_2))
  (set `self.DefaultAirControl` (`CharacterMovementComponent.AirControl` _output_get_2))
  (return))

(fn `Tick Destroy Grapple If Being Too Far`
  (params (distance :type "Float (double-precision)" :default 2000.0))
  (returns (`DidDestroyGrappleHook?` :type Boolean))
  (bind (_valid_ _distance) (`self.Get_DistanceToGrappleProjectile`))
  (if (and (> distance _distance) _valid_)
    (bind _success_ (`self.DestroyGrappleHook`))
    (return _success_)
    (else
      (return false))))

(fn `Tick_AddPullingForce`
  (params (ForceMultiplier :type "Float (double-precision)" :default 500000.0))
  (returns (`Success?` :type Boolean))
  (bind _owningcharactermovementref (`self.OwningCharacterMovementRef`)
    (:`then`
      (`CharacterMovementComponent.AddForce` _owningcharactermovementref (* (`self.Get_DirectionToGrappleProjectile`) (`local.ForceMultiplier`)))
      (return true))
    (:`else`
      (return false))))

(fn `Tick_AddSwingingForce`
  (params (DeltaSecounds :type "Float (double-precision)") (ForceMultiplier :type "Float (double-precision)" :default 20.0))
  (returns (`Success?` :type Boolean))
  (locals (`CalculatedForce (Local)` :type "Float (double-precision)") (`OwningCharacterMovementRef (Local)` :type "CharacterMovementComponent Object Reference"))
  (bind _owningactorref (`self.OwningActorRef`))
  (bind (_returnvalue_x _returnvalue_y _returnvalue_z) (`KismetMathLibrary.BreakVector` (`Actor.K2_GetActorLocation` (`self.OwningActorRef`))))
  (bind (_returnvalue_x_2 _returnvalue_y_2 _returnvalue_z_2) (`KismetMathLibrary.BreakVector` (`Actor.K2_GetActorLocation` (`self.GrappleProjectileRef`))))
  (bind _returnvalue (- (`Actor.K2_GetActorLocation` _owningactorref) (`Actor.K2_GetActorLocation` (`self.GrappleProjectileRef`))))
  (bind _owningcharactermovementref (`self.OwningCharacterMovementRef`)
    (:`then`
      (bind _output_get (set `local.OwningCharacterMovementRef (Local)` _owningcharactermovementref))
      (if (not (and (< (`.Distance` (`self.Get_DistanceToGrappleProjectile`)) (`self.ImagineryRopeLength`)) (`self.bGrounded`)))
        (`CharacterMovementComponent.AddForce` _output_get (select `bool` (> _returnvalue_z_2 (+ _returnvalue_z 200.0)) :`true` (* (* (* (`KismetMathLibrary.Dot_VectorVector` _returnvalue (`Actor.GetVelocity` _owningactorref)) (`KismetMathLibrary.Normal` _returnvalue)) -1.0) (* (`KismetMathLibrary.SafeDivide` 0.01 (`local.DeltaSecounds`)) (`local.ForceMultiplier`)))))
        (return true)))
    (:`else`
      (return false))))

(fn `Tick_CheckIfOnGroundOrInAir`
  (params (KeepSwingingIfLookingAtGrapple :type Boolean :default true))
  (returns (`Success?` :type Boolean))
  (bind _owningcharactermovementref (`self.OwningCharacterMovementRef`)
    (:`then`
      (`|ExecutionSequence`
        (:`then_0`
          (if (and (not (`self.bGrounded`)) (`NavMovementComponent.IsMovingOnGround` _owningcharactermovementref))
            (bind _success_ (`self.OnGroundLanded`))
            (return _success_)))
        (:`then_1`
          (if (and (`self.bGrounded`) (not (`NavMovementComponent.IsMovingOnGround` _owningcharactermovementref)))
            (bind _success__2 (`self.OnAirEntered`))
            (return _success__2)))
        (:`then_2`
          (return true))))
    (:`else`
      (return false))))

(fn `Tick_DebugVariables`
  (params (`IsDebuging?` :type Boolean))
  (if `IsDebuging?`
    (`self.Debug_Variable` "-----------------------------------------------------------------------" "" false true false true 0.0 (struct :`G` 0.102242 :`B` 0.467784 :`A` 1.0))
    (`self.Debug_Reference` "GrappleCableRef:" (`self.GrappleCableRef`) true true false true 0.0 (struct :`G` 0.102242 :`B` 0.467784 :`A` 1.0))
    (`self.Debug_Reference` "GrappleProjectileRef:" (`self.GrappleProjectileRef`) true true false true 0.0 (struct :`G` 0.102242 :`B` 0.467784 :`A` 1.0))
    (`self.Debug_Variable` "GrappleState:" (`|GetEnumeratorNameAsString` (`self.GrappleState`)) true true false true 0.0 (struct :`G` 0.102242 :`B` 0.467784 :`A` 1.0))
    (`self.Debug_Reference` "AimingComponentRef:" (`self.AimingComponentRef`) true true false true 0.0 (struct :`G` 0.102242 :`B` 0.467784 :`A` 1.0))
    (`self.Debug_Reference` "OwningActorRef:" (`self.OwningActorRef`) true true false true 0.0 (struct :`G` 0.102242 :`B` 0.467784 :`A` 1.0))
    (`self.Debug_Variable` "OwningCharacter: InitialPoolingDirection2D:" (`KismetStringLibrary.Conv_VectorToString` (`self.PoolingDirection2D`)) true true false true 0.0 (struct :`G` 0.102242 :`B` 0.467784 :`A` 1.0))
    (`self.Debug_Variable` "OwningCharacter: DefauiltAirControl:" (`KismetStringLibrary.Conv_DoubleToString` (`self.DefaultAirControl`)) true true false true 0.0 (struct :`G` 0.102242 :`B` 0.467784 :`A` 1.0))
    (`self.Debug_Variable` "OwningCharacter: DefaultGravityScale:" (`KismetStringLibrary.Conv_DoubleToString` (`self.DefaultGravityScale`)) true true false true 0.0 (struct :`G` 0.102242 :`B` 0.467784 :`A` 1.0))
    (`self.Debug_Variable` "OwningCharacter: DefaultGroundFriction:" (`KismetStringLibrary.Conv_DoubleToString` (`self.DefaultGroundFriction`)) true true false true 0.0 (struct :`G` 0.102242 :`B` 0.467784 :`A` 1.0))
    (`self.Debug_Reference` "OwningCharacter: OwningCharacterMovementRef:" (`self.OwningCharacterMovementRef`) true true false true 0.0 (struct :`G` 0.102242 :`B` 0.467784 :`A` 1.0))
    (`self.Debug_Reference` "OwningCharacter: OwningCharacterRef:" (`self.OwningCharacterRef`) true true false true 0.0 (struct :`G` 0.102242 :`B` 0.467784 :`A` 1.0))
    (`self.Debug_Variable` "DebugMode:" (`KismetStringLibrary.Conv_BoolToString` (`self.bDebugMode`)) true true false true 0.0 (struct :`G` 0.102242 :`B` 0.467784 :`A` 1.0))
    (`self.Debug_Variable` (`KismetStringLibrary.Concat_StrStr` "------- Debug Component_GrappleHook of " (`KismetSystemLibrary.GetDisplayName` (`self.OwningActorRef`)) " -------") "" false true false true 0.0 (struct :`G` 0.102242 :`B` 0.467784 :`A` 1.0))
    (return)))