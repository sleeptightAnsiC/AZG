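; Projectile actor for the grapple hook movement mechanic, which flies until it exceeds its maximum range.
; On BeginPlay it copies its Velocity and gravity scale variables into the ProjectileMovement component and records its start location.
; Each Tick it measures the straight-line distance from that start and destroys itself once past MaxDistance.
; The graph holds no hit or attach logic.
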(event `self.ReceiveBeginPlay`
  (set `MovementComponent.Velocity` (`self.Velocity`) (`self.ProjectileMovement`))
  (set `ProjectileMovementComponent.ProjectileGravityScale` (`self.ProjectileGravityScale`) (`self.ProjectileMovement`))
  (set `self.StartLocation` (`self.K2_GetActorLocation`)))

(event `self.ReceiveTick`
  (params (DeltaSeconds :type "Float (single-precision)"))
  (if (> (`KismetMathLibrary.Vector_Distance` (`self.StartLocation`) (`self.K2_GetActorLocation`)) (`self.MaxDistance`))
    (`self.K2_DestroyActor` self)))

(fn `UserConstructionScript`)