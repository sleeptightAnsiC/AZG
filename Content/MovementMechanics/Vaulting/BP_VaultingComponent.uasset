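; Actor component that lets its owning Character automatically vault onto ledges while jump and forward inputs are held, or either while falling.
; Each tick drives a NotVaulting/WantsToVault/Vaulting state; a downward trace ahead validates ledge height, walkable slope and capsule clearance.
; Vaulting teleports the character along a lerp, paced by distance and walk speed.
; On completion it multiplies MaxWalkSpeed by a penalty, with no restore here.
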(event `self.ReceiveBeginPlay`
  ;[1 1 1] Set OwningCharacter
  (bind _ascharacter (cast `Character` (`self.GetOwner`))
    (:`then`
      (bind _output_get (set `self.OwningCharacter` _ascharacter))
      (set `self.OwningCharacterMovement` (`Character.CharacterMovement` _output_get)))
    (:`CastFailed`
      (`KismetSystemLibrary.PrintString` "Component_Vaulting: Cast to Character failed" true true (struct :`R` 1.0 :`B` 0.014055 :`A` 1.0)))))

(event `self.ReceiveTick`
  (params (DeltaSeconds :type "Float (single-precision)"))
  ;[1 1 1] Tick Vault Logic
  (`|ExecutionSequence`
    (:`then_0`
      (if (not (`|EnumEquality` (`self.VaultingState`) "NewEnumerator2"))
        (if (or (and (`NavMovementComponent.IsFalling` (`self.OwningCharacterMovement`)) (or (`self.bJumpKeyDown`) (`self.bForwardKeyDown`))) (and (`self.bJumpKeyDown`) (`self.bForwardKeyDown`)))
          (set `self.VaultingState` "NewEnumerator1")
          (else
            (set `self.VaultingState` "NewEnumerator0")))))
    (:`then_1`
      (`self.SwitchOnVaultingState`
        (:`WantsToVault`
          (bind (_result _newendlocation) (`self.CheckIfCanVault`))
          (set `self.EndLocation` _newendlocation)
          (bind _output_get (set `self.bCanVault` _result))
          (if _output_get
            (`self.OnBeginVaulting`)))
        (:`Vaulting`
          (`self.TickVaultingLogic` DeltaSeconds))))))

(event `InputAxis|MoveForward` :consume false :overrideparent false
  (params (AxisValue :type "Float (single-precision)"))
  ;[1 1 1] Input Logic
  (set `self.bForwardKeyDown` (> AxisValue 0.0)))

(event `InputAction|Jump` :consume false :overrideparent false
  (params (Key :type "Key Structure"))
  ;[1 1 1] Input Logic
  (:`Pressed`
    (set `self.bJumpKeyDown` true))
  (:`Released`
    (set `self.bJumpKeyDown` false)))

(fn `CapsuleCollisionCast`
  (params (Center :type "Vector Structure") (HalfHeight :type "Float (double-precision)") (Radius :type "Float (double-precision)") (DrawDebug :type Boolean))
  (returns (`CapsuleCollided?` :type Boolean))
  (`|ExecutionSequence`
    (:`then_0`
      ;[1 1 1] Debug
      (if (`local.DrawDebug`)
        (`KismetSystemLibrary.DrawDebugCapsule` (`local.Center`) (`local.HalfHeight`) (`local.Radius`) (struct) (struct :`R` 0.119538 :`G` 0.467784 :`B` 0.456411 :`A` 1.0) 0.0 3.0)))
    (:`then_1`
      ;[1 1 1] Check If Capsule Overlap Any Actor
      (bind (_outactors _returnvalue) (`KismetSystemLibrary.CapsuleOverlapActors` (`local.Center`) (`local.Radius`) (`local.HalfHeight`) (`|MakeArray` "ObjectTypeQuery1" "ObjectTypeQuery2" "ObjectTypeQuery4" "ObjectTypeQuery5" "ObjectTypeQuery6" :!type "EObjectTypeQuery Enum") "/Script/Engine.Actor" (`|MakeArray` (`self.OwningCharacter`) :!type "Actor Object Reference")))
      (return _returnvalue))))

(fn `CheckIfCanVault`
  (returns (Result :type Boolean) (NewEndLocation :type "Vector Structure"))
  (locals (`OwningCharacterCapsule (Local)` :type "CapsuleComponent Object Reference"))
  (bind _owningcharacter (`self.OwningCharacter`))
  (bind _returnvalue (`CapsuleComponent.GetScaledCapsuleHalfHeight` (`local.OwningCharacterCapsule (Local)`)))
  (bind _returnvalue_2 (+ (`Actor.K2_GetActorLocation` _owningcharacter) (* (`Actor.GetActorForwardVector` _owningcharacter) 80.0)))
  (if (not (`|EnumEquality` (`self.VaultingState`) "NewEnumerator2"))
    (set `local.OwningCharacterCapsule (Local)` (`Character.CapsuleComponent` (`self.OwningCharacter`)))
    (bind (_outhit _returnvalue_3) (`KismetSystemLibrary.LineTraceSingle` (+ _returnvalue_2 (`KismetMathLibrary.MakeVector` 0.0 0.0 (+ _returnvalue 0.0))) (- _returnvalue_2 (`KismetMathLibrary.MakeVector` 0.0 0.0 _returnvalue)) "TraceTypeQuery1" false (`|MakeArray` (`self.OwningCharacter`) :!type "Actor Object Reference")))
    (if _returnvalue_3
      (bind (_result _endinglocation) (`self.CheckIfCanVaultToHit` (`local.OwningCharacterCapsule (Local)`) _outhit))
      (`KismetSystemLibrary.PrintString` (`KismetStringLibrary.Conv_BoolToString` _result) true true (struct :`R` 0.119538 :`G` 0.467784 :`B` 0.456411 :`A` 1.0) 0.0)
      (return _result _endinglocation)
      (else
        (return false (0.0 0.0 0.0))))
    (else
      (return false (0.0 0.0 0.0)))))

(fn `CheckIfCanVaultToHit`
  (params (Capsule :type "CapsuleComponent Object Reference") (Hit :type "HitResult Structure"))
  (returns (Result :type Boolean) (EndingLocation :type "Vector Structure"))
  (locals (`EndingLocation (Local)` :type "Vector Structure" :default (0.0 0.0 0.0)))
  (bind _capsule (`local.Capsule`))
  (bind _returnvalue (`CapsuleComponent.GetScaledCapsuleRadius` _capsule))
  (bind (_bblockinghit _binitialoverlap _time _distance _location _impactpoint _normal _impactnormal _physmat _hitactor _hitcomponent _hitbonename _bonename _hititem _elementindex _faceindex _tracestart _traceend) (`GameplayStatics.BreakHitResult` (`local.Hit`)))
  (bind _returnvalue_2 (- (.z _location) (.z _traceend)))
  (`|ExecutionSequence`
    (:`then_0`
      ;[1 1 1] Make Sure That The Ledge Is At Inpropriete Height
      (`KismetSystemLibrary.PrintString` (`KismetStringLibrary.Conv_DoubleToString` _returnvalue_2) true true (struct :`R` 0.119538 :`G` 0.467784 :`B` 0.456411 :`A` 1.0) 0.0)
      (if (not (`KismetMathLibrary.InRange_FloatFloat` _returnvalue_2 (`self.MinVaultingHeight`) (`self.MaxVaultingHeight`)))
        (return false (0.0 0.0 0.0))))
    (:`then_1`
      ;[1 1 1] Make Sure That Surface Is Wakable
      (if (< (.z (`.Normal` (`GameplayStatics.BreakHitResult` (`local.Hit`)))) (`CharacterMovementComponent.K2_GetWalkableFloorZ` (`self.OwningCharacterMovement`)))
        (return false (0.0 0.0 0.0))))
    (:`then_2`
      ;[1 1 1] Make Sure That There Is A Space For Character
      (bind _output_get (set `local.EndingLocation (Local)` (+ (`.Location` (`GameplayStatics.BreakHitResult` (`local.Hit`))) (`KismetMathLibrary.MakeVector` 0.0 0.0 (`CapsuleComponent.GetScaledCapsuleHalfHeight` (`local.Capsule`))))))
      (bind _capsulecollided_ (`self.CapsuleCollisionCast` (+ _output_get (`KismetMathLibrary.MakeVector` 0.0 0.0 _returnvalue)) (`CapsuleComponent.GetScaledCapsuleHalfHeight` _capsule) _returnvalue))
      (if _capsulecollided_
        (return false (0.0 0.0 0.0))))
    (:`then_3`
      (return true (`local.EndingLocation (Local)`)))))

(fn `Get_CanVault`
  (returns (CanVault :type Boolean))
  (return (`self.bCanVault`)))

(fn `OnBeginVaulting`
  (returns (`DidStartVaulting?` :type Boolean))
  (if (`self.bCanVault`)
    (set `self.Progress` 0.0)
    (set `self.StartLocation` (`Actor.K2_GetActorLocation` (`self.OwningCharacter`)))
    (set `self.VaultingState` "NewEnumerator2")
    (return true)
    (else
      (return false))))

(fn `TickVaultingLogic`
  (params (DeltaSeconds :type "Float (double-precision)"))
  (bind _owningcharactermovement (`self.OwningCharacterMovement`))
  (`|ExecutionSequence`
    (:`then_0`
      (bind _output_get (set `self.Progress` (`KismetMathLibrary.FClamp` (+ (`self.Progress`) (* (`local.DeltaSeconds`) (* (`KismetMathLibrary.MapRangeClamped` (`KismetMathLibrary.Vector_Distance` (`self.StartLocation`) (`self.EndLocation`)) (`self.MinVaultingHeight`) (`self.MaxVaultingHeight`) 3.0 1.0) (`self.VaultSpeedMultiplier`) (`KismetMathLibrary.MapRangeClamped` (`CharacterMovementComponent.MaxWalkSpeed` (`self.OwningCharacterMovement`)) 1100.0 300.0 1.0 3.0)))))))
      (`Actor.K2_SetActorLocation` (`self.OwningCharacter`) (`KismetMathLibrary.VLerp` (`self.StartLocation`) (`self.EndLocation`) _output_get) false true))
    (:`then_1`
      (if (>= (`self.Progress`) 1.0)
        (set `self.VaultingState` "NewEnumerator0")
        (set `CharacterMovementComponent.MaxWalkSpeed` (* (`CharacterMovementComponent.MaxWalkSpeed` _owningcharactermovement) (`self.OnVaultMovementSpeedPenality`)) _owningcharactermovement)))
    (:`then_2`
      (return))))