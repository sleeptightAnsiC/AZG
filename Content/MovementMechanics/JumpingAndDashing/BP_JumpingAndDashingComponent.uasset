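; Character component that turns the jump key into a jump or a cooldown-gated dash, depending on movement input direction.
; Classifies movement state by grounding, velocity and capsule height, then looks up that state's abilities and strengths in a map validated on BeginPlay.
; Jumps are static, adaptive (hold-time) or charged; charge builds on Tick and fires on key release if the state is unchanged.
; Tick also prints debug values.
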(event `self.ReceiveBeginPlay`
  (`self.Set_OwningCharacter` (`self.GetOwner`))
  (`self.CheckIfContainsEveryKey` (`self.EsentialParameters`) "EsentialParameters"))

(event `self.ReceiveTick`
  (params (DeltaSeconds :type "Float (single-precision)"))
  (`self.Tick_IncreaseLaunchForceMultiplier` DeltaSeconds (`self.MaxLaunchForceMultiplier`) (`self.ForceMultiplierIncreasePerSecond`))
  (`self.DebugVariables` true))

(event `JumpKeyDown`
  (bind _new_jumping_dashingstate (`self.Find_Jumping&DashingState`))
  (set `self.Jumping&DashingState` _new_jumping_dashingstate)
  (bind (_newlaunchtype _newlaunchdirection) (`self.Find_LaunchTypeAndDirection` 0.5))
  (switch `/Game/MovementMechanics/JumpingAndDashing/ELaunchType` _newlaunchtype
    (:`NewEnumerator0`
      (`self.OnJump` (`self.Jumping&DashingState`)))
    (:`NewEnumerator1`
      (`/Engine/EditorBlueprintResources/StandardMacros.DoOnce` false :!label _label
        (:`Completed`
          (bind _diddash_ (`self.OnDash` _newlaunchdirection (`self.Jumping&DashingState`)))
          (if _diddash_
            (`KismetSystemLibrary.Delay` (`self.DashCooldown`))
            (goto _label :!via `Reset`)
            (else
              (goto _label :!via `Reset`))))))))

(event `JumpKeyUp`
  (`self.OnChargedJump` (`self.Jumping&DashingState`))
  (`Character.StopJumping` (`self.CharacterRef`)))

(fn `CheckIfContainsEveryKey`
  (params (TargetMap :type "Map of /Game/MovementMechanics/JumpingAndDashing/EJumpingAndDashingState Enum to /Game/MovementMechanics/JumpingAndDashing/FJumpingAndDashingParameters Structure (by ref)") (MapName :type String))
  (returns (`Valid?` :type Boolean))
  (locals (`(Local) Valid?` :type Boolean :default true))
  (bind _enumvalue (foreach `/Game/MovementMechanics/JumpingAndDashing/EJumpingAndDashingState` false)
    (:`LoopBody`
      (if (not (`BlueprintMapLibrary.Map_Contains` TargetMap _enumvalue))
        (set `local.(Local) Valid?` false)
        (bind _returnvalue (`KismetStringLibrary.Concat_StrStr` "ERROR!   " (`KismetSystemLibrary.GetDisplayName` self) ": " MapName " map (E_JumpingAndDashingState) does not contain key: " (`|GetEnumeratorNameAsString` _enumvalue)))
        (`KismetSystemLibrary.PrintString` _returnvalue true true (struct :`R` 0.779167 :`B` 0.048325 :`A` 1.0) 10.0 (`KismetStringLibrary.Conv_StringToName` _returnvalue))))
    (:`then`
      (return (`local.(Local) Valid?`)))))

(fn `DebugVariables`
  (params (Debug :type Boolean :default true))
  (if Debug
    (bind (_newlaunchtype _newlaunchdirection) (`self.Find_LaunchTypeAndDirection` 0.5))
    (`self.Debug_Variable` "Jumping&DashingState: " (`|GetEnumeratorNameAsString` _newlaunchtype) true true false true 0.0 (struct :`R` 0.006995 :`B` 0.450786 :`A` 1.0))
    (`self.Debug_Variable` "LaunchDirection: " (`KismetStringLibrary.Conv_VectorToString` _newlaunchdirection) true true false true 0.0 (struct :`R` 0.006995 :`B` 0.450786 :`A` 1.0))
    (`self.Debug_Variable` "IsWaitingForChargedJump?: " (`KismetStringLibrary.Conv_BoolToString` (`self.bWaitingForChargedJump`)) true true false true 0.0 (struct :`R` 0.006995 :`B` 0.450786 :`A` 1.0))
    (`self.Debug_Variable` "LastRightAxisValue: " (`KismetStringLibrary.Conv_DoubleToString` (`self.LastRightAxisValue`)) true true false true 0.0 (struct :`R` 0.006995 :`B` 0.450786 :`A` 1.0))
    (`self.Debug_Variable` "LastForwardAxisValue: " (`KismetStringLibrary.Conv_DoubleToString` (`self.LastForwardAxisValue`)) true true false true 0.0 (struct :`R` 0.006995 :`B` 0.450786 :`A` 1.0))
    (`self.Debug_Variable` "LaunchForceMultiplier: " (`KismetStringLibrary.Conv_DoubleToString` (`self.LaunchForceMultiplier`)) true true false true 0.0 (struct :`R` 0.006995 :`B` 0.450786 :`A` 1.0))
    (return)
    (else
      (return))))

(fn `Find_Jumping&DashingState`
  (returns (`New_Jumping&DashingState` :type "/Game/MovementMechanics/JumpingAndDashing/EJumpingAndDashingState Enum"))
  (locals (`IsMoving (Local)` :type Boolean))
  (set `local.IsMoving (Local)` (not (== (`MovementComponent.Velocity` (`self.CharacterMovementRef`)) (0.0 0.0 0.0) :`ErrorTolerance` 0.1)))
  (if (not (`NavMovementComponent.IsMovingOnGround` (`self.CharacterMovementRef`)))
    (if (`local.IsMoving (Local)`)
      (return "NewEnumerator1")
      (else
        (return "NewEnumerator5")))
    (elif (== (`self.Default Capsule Half Height`) (`CapsuleComponent.CapsuleHalfHeight` (`Character.CapsuleComponent` (`self.CharacterRef`))))
      (if (`local.IsMoving (Local)`)
        (return "NewEnumerator2")
        (else
          (return "NewEnumerator6")))
      (elif (`local.IsMoving (Local)`)
        (return "NewEnumerator3")
        (else
          (return "NewEnumerator7"))))))

(fn `Find_LaunchTypeAndDirection`
  (params (MinDotProductToJump :type "Float (double-precision)" :default 0.5))
  (returns (NewLaunchType :type "/Game/MovementMechanics/JumpingAndDashing/ELaunchType Enum") (NewLaunchDirection :type "Vector Structure"))
  (bind _characterref (`self.CharacterRef`))
  (bind _returnvalue (`Actor.GetActorForwardVector` _characterref))
  (bind _returnvalue_2 (`KismetMathLibrary.Normal` (+ (* (`Actor.GetActorRightVector` _characterref) (`self.LastRightAxisValue`)) (* _returnvalue (`self.LastForwardAxisValue`)))))
  (return (select `bool` (or (and (== (`self.LastRightAxisValue`) 0.0) (== (`self.LastForwardAxisValue`) 0.0)) (< MinDotProductToJump (`KismetMathLibrary.Dot_VectorVector` _returnvalue_2 _returnvalue))) :`false` "NewEnumerator1" :`true` "NewEnumerator0" :!type "/Game/MovementMechanics/JumpingAndDashing/ELaunchType Enum") _returnvalue_2))

(fn `OnChargedJump`
  (params (JumpingAndDashingState :type "/Game/MovementMechanics/JumpingAndDashing/EJumpingAndDashingState Enum (by ref)"))
  (returns (`DidChargedJump?` :type Boolean))
  (bind _characterref (`self.CharacterRef`))
  (if (`self.bWaitingForChargedJump`)
    (set `self.bWaitingForChargedJump` false)
    (bind _new_jumping_dashingstate (`self.Find_Jumping&DashingState`))
    (if (`|EnumEquality` _new_jumping_dashingstate JumpingAndDashingState)
      (set `CharacterMovementComponent.JumpZVelocity` (* (`KismetMathLibrary.NormalizeToRange` (`self.LaunchForceMultiplier`) (`self.MinLaunchForceMultiplier`) (`self.MaxLaunchForceMultiplier`)) (`.JumpStrength_13_14635411427ADF2EE5211EBF60CCEE60` (break `/Game/MovementMechanics/JumpingAndDashing/FJumpingAndDashingParameters` (`BlueprintMapLibrary.Map_Find` (`self.EsentialParameters`) JumpingAndDashingState)))) (`self.CharacterMovementRef`))
      (set `Character.JumpMaxHoldTime` 0.0 _characterref)
      (`Character.Jump` _characterref)
      (return true)
      (else
        (return false)))
    (else
      (return false))))

(fn `OnDash`
  (params (DashDirection :type "Vector Structure") (JumpingAndDashingState :type "/Game/MovementMechanics/JumpingAndDashing/EJumpingAndDashingState Enum (by ref)"))
  (returns (`DidDash?` :type Boolean))
  (bind (_candash_ _dashstrength) (break `/Game/MovementMechanics/JumpingAndDashing/FJumpingAndDashingParameters` (`BlueprintMapLibrary.Map_Find` (`self.EsentialParameters`) JumpingAndDashingState)))
  (if _candash_
    (`Character.LaunchCharacter` (`self.CharacterRef`) (* (+ DashDirection (0.0 0.0 0.15)) _dashstrength) false false)
    (return true)
    (else
      (return false))))

(fn `OnJump`
  (params (JumpingAndDashingState :type "/Game/MovementMechanics/JumpingAndDashing/EJumpingAndDashingState Enum (by ref)"))
  (returns (`DidJump?` :type Boolean) (JumpType :type "/Game/MovementMechanics/JumpingAndDashing/EJumpType Enum"))
  (bind _characterref (`self.CharacterRef`))
  (bind _characterref_2 (`self.CharacterRef`))
  (bind (_candash_ _dashstrength _canjump_ _jumptype _jumpstrength _jumpholdtime) (break `/Game/MovementMechanics/JumpingAndDashing/FJumpingAndDashingParameters` (`BlueprintMapLibrary.Map_Find` (`self.EsentialParameters`) JumpingAndDashingState)))
  (if _canjump_
    (switch `/Game/MovementMechanics/JumpingAndDashing/EJumpType` _jumptype
      (:`NewEnumerator0`
        (set `CharacterMovementComponent.JumpZVelocity` _jumpstrength (`self.CharacterMovementRef`))
        (set `Character.JumpMaxHoldTime` 0.0 _characterref)
        (`Character.Jump` _characterref)
        (return true "NewEnumerator0"))
      (:`NewEnumerator1`
        (set `CharacterMovementComponent.JumpZVelocity` _jumpstrength (`self.CharacterMovementRef`))
        (set `Character.JumpMaxHoldTime` _jumpholdtime _characterref_2)
        (`Character.Jump` _characterref_2)
        (return true "NewEnumerator1"))
      (:`NewEnumerator2`
        (set `self.LaunchForceMultiplier` (`self.MinLaunchForceMultiplier`))
        (set `self.bWaitingForChargedJump` true)
        (return false "NewEnumerator2")))
    (else
      (return false _jumptype))))

(fn `Set_OwningCharacter`
  (params (CharacterRef :type "Actor Object Reference"))
  (returns (`Success?` :type Boolean))
  (bind _ascharacter (cast `Character` CharacterRef)
    (:`then`
      (bind _output_get (set `self.CharacterRef` _ascharacter))
      (set `self.CharacterMovementRef` (`Character.CharacterMovement` _output_get))
      (set `self.Default Capsule Half Height` (`CapsuleComponent.CapsuleHalfHeight` (`Character.CapsuleComponent` _output_get)))
      (return true))
    (:`CastFailed`
      (`self.Throw_CastFailedError` "Character" CharacterRef)
      (return false))))

(fn `Tick_IncreaseLaunchForceMultiplier`
  (params (DeltaSecounds :type "Float (double-precision)") (MaxLaunchForceMultiplier :type "Float (double-precision)" :default 2.0) (ForceMultiplierIncreasePerSecond :type "Float (double-precision)" :default 1.0))
  (returns (`IsChargingJump?` :type Boolean))
  (bind _maxlaunchforcemultiplier (`local.MaxLaunchForceMultiplier`))
  (bind _returnvalue (+ (`self.LaunchForceMultiplier`) (* (`self.ForceMultiplierIncreasePerSecond`) (`local.DeltaSecounds`))))
  (if (`self.bWaitingForChargedJump`)
    (set `self.LaunchForceMultiplier` (select `bool` (> _returnvalue _maxlaunchforcemultiplier) :`false` _returnvalue :`true` _maxlaunchforcemultiplier))
    (return true)
    (else
      (return false))))